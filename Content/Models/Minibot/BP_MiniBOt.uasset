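; BP_MiniBOt is a hovering minibot that also serves as the view target for the player's range ability selection screen.
; Looping timelines bob it up and down and spin its propeller by nudging world transforms on each update.
; CameraEvent blends the view to the bot, snaps it to a fixed height and stops the bobbing.
; It also switches to UI-only input with a cursor and shows randomized abilities through the cached player's main widget.
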(event `TwistProp`
  (bind _propeller (`self.propeller`))
  (bind (_returnvalue_roll _returnvalue_pitch _returnvalue_yaw) (`KismetMathLibrary.BreakRotator` (`SceneComponent.K2_GetComponentRotation` _propeller)))
  ; Move Bot
  (`Timeline|Twist` :!via `PlayFromStart`
    (:`Update`
      (`SceneComponent.K2_SetWorldRotation` _propeller (`KismetMathLibrary.MakeRotator` 0.0 0.0 (+ _returnvalue_yaw 10.0)) false false))
    (:`Finished`
      (`self.TwistProp`))))

(event `self.ReceiveBeginPlay`
  (`|ExecutionSequence`
    (:`then_0`
      (`self.Up/Down`)
      (`self.TwistProp`))
    (:`then_1`
      (bind _asbp_player_base (cast `/Game/Blueprints/Characters/BP_Player_Base` (`Controller.K2_GetPawn` (`GameplayStatics.GetPlayerController` 0))))
      (set `self.BP_Character` _asbp_player_base))))

(event `Up/Down`
  (bind _defaultsceneroot (`self.DefaultSceneRoot`))
  (bind (_returnvalue_x _returnvalue_y _returnvalue_z) (`KismetMathLibrary.BreakVector` (`SceneComponent.K2_GetComponentLocation` _defaultsceneroot)))
  ; Move Bot
  (`Timeline|TimeUp` :!via `PlayFromStart` :!label _label
    (:`Update`
      (`SceneComponent.K2_SetWorldLocation` _defaultsceneroot (`KismetMathLibrary.MakeVector` _returnvalue_x _returnvalue_y (+ _returnvalue_z 0.3)) false false))
    (:`Finished`
      (`self.Down`))))

(event `Pause`
  (bind _defaultsceneroot (`self.DefaultSceneRoot`))
  (bind (_returnvalue_x _returnvalue_y _returnvalue_z) (`KismetMathLibrary.BreakVector` (`SceneComponent.K2_GetComponentLocation` _defaultsceneroot)))
  ; Move Bot
  (`|ExecutionSequence`
    (:`then_0`
      (goto _label :!via `Stop`))
    (:`then_1`
      (`Timeline|TimeDown` :!via `Stop` :!label _label_2
        (:`Update`
          (`SceneComponent.K2_SetWorldLocation` _defaultsceneroot (`KismetMathLibrary.MakeVector` _returnvalue_x _returnvalue_y (- _returnvalue_z 0.3)) false false))
        (:`Finished`
          (`self.Up/Down`))))))

(event `Down`
  ; Move Bot
  (goto _label_2 :!via `PlayFromStart`))

(event `CameraEvent`
  (bind _returnvalue (`GameplayStatics.GetPlayerController` 0))
  (bind _defaultsceneroot (`self.DefaultSceneRoot`))
  (bind (_returnvalue_x _returnvalue_y) (`KismetMathLibrary.BreakVector` (`SceneComponent.K2_GetComponentLocation` _defaultsceneroot)))
  (bind _wbp_rangeabilities (`/Game/Interface/WBP_MainWIdget.WBP_RangeAbilities` (`/Game/Blueprints/Characters/BP_Player_Base.MainWidget` (`self.BP_Character`))))
  (`PlayerController.SetViewTargetWithBlend` _returnvalue self 0.5 "VTBlend_Linear" 0.0 false)
  (`WidgetBlueprintLibrary.SetInputMode_UIOnlyEx` _returnvalue _wbp_rangeabilities)
  (set `PlayerController.bShowMouseCursor` true _returnvalue)
  (`Widget.SetVisibility` _wbp_rangeabilities "Visible")
  (`SceneComponent.K2_SetWorldLocation` _defaultsceneroot (`KismetMathLibrary.MakeVector` _returnvalue_x _returnvalue_y -1640.0) false false)
  (`self.Pause`)
  (`/Game/Interface/WBP_RangeAbilities.GetRandomAbilities` _wbp_rangeabilities))

(fn `UserConstructionScript`)
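; BP_Metal_Door is an automatic metal door that reacts to the player character or enemies entering and leaving its trigger Box.
; On overlap it restarts a Timeline, whose completion plays the skeletal door's opening animation.
; On exit it plays the closing animation and enables collision on Block.
; The delayed step that would disable Block's collision is disconnected and never runs.
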(event `self.Box.OnComponentBeginOverlap`
  (params (OverlappedComponent :type "PrimitiveComponent Object Reference") (OtherActor :type "Actor Object Reference") (OtherComp :type "PrimitiveComponent Object Reference") (OtherBodyIndex :type Integer) (bFromSweep :type Boolean) (SweepResult :type "HitResult Structure (by ref)"))
  (`|ExecutionSequence`
    (:`then_0`
      (cast `/Game/ThirdPerson/Blueprints/BP_ThirdPersonCharacter` OtherActor)
      (`Timeline|Timeline` :!via `PlayFromStart` :!label _label
        (:`Finished`
          (`SkeletalMeshComponent.PlayAnimation` (`self.SM_Door`) "/Game/Models/Door/door_01__3__Anim.door_01__3__Anim" false))))
    (:`then_1`
      (cast `/Game/Blueprints/AI/Enemys/BP_Enemy_Base` OtherActor)
      (goto _label :!via `PlayFromStart`))))

(event `self.Box.OnComponentEndOverlap`
  (params (OverlappedComponent :type "PrimitiveComponent Object Reference") (OtherActor :type "Actor Object Reference") (OtherComp :type "PrimitiveComponent Object Reference") (OtherBodyIndex :type Integer))
  (`|ExecutionSequence`
    (:`then_0`
      (cast `/Game/ThirdPerson/Blueprints/BP_ThirdPersonCharacter` OtherActor))
    (:`then_1`
      (cast `/Game/Blueprints/AI/Enemys/BP_Enemy_Base` OtherActor)))
  (`SkeletalMeshComponent.PlayAnimation` (`self.SM_Door`) "/Game/Models/Door/MoreDoor/door_01__4_anim_door_01_close.door_01__4_anim_door_01_close" false)
  (`PrimitiveComponent.SetCollisionEnabled` (`self.Block`) "QueryAndPhysics"))

(fn `UserConstructionScript`)
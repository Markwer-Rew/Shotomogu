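; Glass door actor that plays a skeletal door animation when another actor overlaps its Open trigger.
; The only working logic plays a clip named as the close animation, once per overlap with a valid actor.
; Disconnected leftovers include an OpenGlassDoor timeline, Box offsets from the transform cached at BeginPlay, and a delayed collision toggle.
; The Box end-overlap event is empty.
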(event `self.ReceiveBeginPlay`
  (set `self.Location` (`self.GetTransform`)))

(event `self.Open.OnComponentBeginOverlap`
  (params (OverlappedComponent :type "PrimitiveComponent Object Reference") (OtherActor :type "Actor Object Reference") (OtherComp :type "PrimitiveComponent Object Reference") (OtherBodyIndex :type Integer) (bFromSweep :type Boolean) (SweepResult :type "HitResult Structure (by ref)"))
  (`/Engine/EditorBlueprintResources/StandardMacros.IsValid` OtherActor
    (:`Is Valid`
      (`SkeletalMeshComponent.PlayAnimation` (`self. SM_Door`) "/Game/Models/Door/MoreDoor/door_02__2_anim_door_close.door_02__2_anim_door_close" false))))

(event `self.Box.OnComponentEndOverlap`
  (params (OverlappedComponent :type "PrimitiveComponent Object Reference") (OtherActor :type "Actor Object Reference") (OtherComp :type "PrimitiveComponent Object Reference") (OtherBodyIndex :type Integer)))

(fn `UserConstructionScript`)
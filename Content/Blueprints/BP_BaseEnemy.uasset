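; BP_BaseEnemy is a base enemy that takes damage and moves toward the player character when it comes within range.
; An overlap with its sphere collision casts the other actor to BP_ThirdPersonCharacter and starts an AI MoveTo targeting it, stopping on overlap.
; AnyDamage subtracts from a clamped Health value and destroys the actor when it reaches zero.
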(event `self.ReceiveAnyDamage`
  (params (Damage :type "Float (single-precision)") (DamageType :type "DamageType Object Reference") (InstigatedBy :type "Controller Object Reference") (DamageCauser :type "Actor Object Reference"))
  (bind _output_get (set `self.Health` (`KismetMathLibrary.FClamp` (- (`self.Health`) Damage) 0.0 100.0)))
  (if (<= _output_get 0.0)
    (`self.K2_DestroyActor`)))

(event `self.SphereCollision.OnComponentBeginOverlap`
  (params (OverlappedComponent :type "PrimitiveComponent Object Reference") (OtherActor :type "Actor Object Reference") (OtherComp :type "PrimitiveComponent Object Reference") (OtherBodyIndex :type Integer) (bFromSweep :type Boolean) (SweepResult :type "HitResult Structure (by ref)"))
  (bind _asbp_third_person_character (cast `/Game/ThirdPerson/Blueprints/BP_ThirdPersonCharacter` OtherActor))
  (`|AIMoveTo` null (`self.K2_GetActorLocation` _asbp_third_person_character) _asbp_third_person_character 5.0 true))

(fn `UserConstructionScript`)
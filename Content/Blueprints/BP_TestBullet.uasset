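; BP_TestBullet is a test bullet actor that applies a configurable Gameplay Ability System effect to actors it hits.
; On sphere hit, it builds a spec from EffectClass, sets a tag-based SetByCaller magnitude and applies it to the target's Ability System Component.
; After a short delay it removes all stacks of that effect.
; A BeginPlay timer destroys the bullet after a fixed lifetime; the end-overlap event is empty, leaving its removal logic disconnected.
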(event `self.Sphere.OnComponentHit`
  (params (HitComponent :type "PrimitiveComponent Object Reference") (OtherActor :type "Actor Object Reference") (OtherComp :type "PrimitiveComponent Object Reference") (NormalImpulse :type "Vector Structure") (Hit :type "HitResult Structure (by ref)"))
  (bind _returnvalue (`AbilitySystemBlueprintLibrary.GetAbilitySystemComponent` OtherActor))
  (`/Engine/EditorBlueprintResources/StandardMacros.IsValid` _returnvalue
    (:`Is Valid`
      (bind _returnvalue_2 (`AbilitySystemBlueprintLibrary.MakeSpecHandleByClass` (`self.EffectClass`) null self))
      (bind _returnvalue_3 (`AbilitySystemBlueprintLibrary.AssignTagSetByCallerMagnitude` _returnvalue_2 (`self.EffectMagnitudeDataTag`) (`self.EffectMagnitudeValue`)))
      (`AbilitySystemComponent.BP_ApplyGameplayEffectSpecToSelf` _returnvalue _returnvalue_3)
      (`KismetSystemLibrary.Delay` 0.2)
      (`AbilitySystemComponent.RemoveActiveGameplayEffectBySourceEffect` _returnvalue (`self.EffectClass`) null -1))))

(event `self.Sphere.OnComponentEndOverlap`
  (params (OverlappedComponent :type "PrimitiveComponent Object Reference") (OtherActor :type "Actor Object Reference") (OtherComp :type "PrimitiveComponent Object Reference") (OtherBodyIndex :type Integer)))

(event `self.ReceiveBeginPlay`
  (`KismetSystemLibrary.K2_SetTimerDelegate` (delegate `Destroy`) 2.0))

(event `Destroy`
  (`self.K2_DestroyActor`))

(fn `UserConstructionScript`)
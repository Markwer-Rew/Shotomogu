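; GA_Hook is a gameplay ability that fires a grappling hook from BP_Player_Base's follow camera.
; A forward visibility trace finds the anchor; on a hit, the character switches to Flying, shows its Cable to the impact point and commits the cooldown.
; One large force pulls toward the anchor, skewed along the actor's right vector.
; The ability ends after a short delay or immediately on a miss, restoring Walking and hiding the cable.
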(event `self.K2_ActivateAbility`
  (bind _asbp_player_base (`self.GetChar`))
  (bind _cable (`/Game/Blueprints/Characters/BP_Player_Base.Cable` _asbp_player_base))
  (bind _charactermovement (`Character.CharacterMovement` _asbp_player_base))
  (bind _followcamera (`/Game/Blueprints/Characters/BP_Player_Base.FollowCamera` _asbp_player_base))
  (bind _returnvalue (`SceneComponent.K2_GetComponentLocation` _followcamera))
  (bind (_outhit _returnvalue_2) (`KismetSystemLibrary.LineTraceSingle` :`Start` _returnvalue :`End` (+ _returnvalue (* (`SceneComponent.GetForwardVector` _followcamera) 3000.0)) :`TraceChannel` "TraceTypeQuery1" :`DrawDebugType` "ForDuration"))
  (if _returnvalue_2
    (`CharacterMovementComponent.SetMovementMode` _charactermovement "MOVE_Flying" 0)
    (`SceneComponent.SetVisibility` _cable true false)
    (bind (_bblockinghit _binitialoverlap _time _distance _location _impactpoint) (`GameplayStatics.BreakHitResult` _outhit))
    (set `CableComponent.EndLocation` (`KismetMathLibrary.InverseTransformLocation` (`Actor.GetTransform` _asbp_player_base) _impactpoint) _cable)
    (`CharacterMovementComponent.AddForce` _charactermovement (* (`KismetMathLibrary.Normal` (+ (`KismetMathLibrary.GetDirectionUnitVector` (`Actor.K2_GetActorLocation` _asbp_player_base) _impactpoint) (* (* (`Actor.GetActorRightVector` _asbp_player_base) (`self.Float`)) 0.7))) 10000000.0))
    (`self.K2_CommitAbilityCooldown` false)
    (`KismetSystemLibrary.Delay` 0.6)
    (`self.K2_EndAbility`)
    (else
      (`self.K2_EndAbility`))))

(event `self.K2_OnEndAbility`
  (params (bWasCancelled :type Boolean))
  (bind _asbp_player_base (`self.GetChar`))
  (`CharacterMovementComponent.SetMovementMode` (`Character.CharacterMovement` _asbp_player_base) "MOVE_Walking" 0)
  (`SceneComponent.SetVisibility` (`/Game/Blueprints/Characters/BP_Player_Base.Cable` _asbp_player_base) false false))

(fn `GetChar`
  (returns (`AsBP Player Base` :type "/Game/Blueprints/Characters/BP_Player_Base Object Reference"))
  (bind _asbp_player_base (cast `/Game/Blueprints/Characters/BP_Player_Base` (`self.GetAvatarActorFromActorInfo`)))
  (return _asbp_player_base))

(fn `GetFollowCamera`
  (returns (FollowCamera :type "CameraComponent Object Reference"))
  (return null))
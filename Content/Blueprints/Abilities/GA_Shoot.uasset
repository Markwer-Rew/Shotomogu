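; GA_Shoot is a gameplay ability that fires a hitscan shot from the player's follow camera.
; On activation it line traces along the camera's forward vector on the Visibility channel, with debug drawing.
; It reports a damage event and applies fixed damage to the hit actor, then commits the cooldown and ends.
; The trace result is never checked, and cooldown is committed only after the shot.
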(event `self.K2_ActivateAbility`
  (bind _followcamera (`self.GetFollowCamera`))
  (bind _returnvalue (`SceneComponent.K2_GetComponentLocation` _followcamera))
  (bind _outhit (`KismetSystemLibrary.LineTraceSingle` :`Start` _returnvalue :`End` (+ _returnvalue (* (`SceneComponent.GetForwardVector` _followcamera) (`self.LineTraceLength`))) :`TraceChannel` "TraceTypeQuery1" :`DrawDebugType` "ForDuration"))
  (bind (_bblockinghit _binitialoverlap _time _distance _location _impactpoint _normal _impactnormal _physmat _hitactor) (`GameplayStatics.BreakHitResult` _outhit))
  (`AISense_Damage.ReportDamageEvent` _hitactor null 1.0)
  (`GameplayStatics.ApplyDamage` _hitactor 45.0 null null "/Script/Engine.DamageType")
  (`self.K2_CommitAbilityCooldown` false)
  (`self.K2_EndAbility`))

(fn `GetFollowCamera`
  (returns (FollowCamera :type "CameraComponent Object Reference"))
  (bind _asbp_player_base (cast `/Game/Blueprints/Characters/BP_Player_Base` (`self.GetAvatarActorFromActorInfo`)))
  (return (`/Game/Blueprints/Characters/BP_Player_Base.FollowCamera` _asbp_player_base)))
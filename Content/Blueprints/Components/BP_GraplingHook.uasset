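; Grappling hook component that pulls a character toward a grab point and releases it on demand.
; Grab sets movement to Flying, shows the cable with its end at the point in actor-local space, and applies a large force toward it.
; The pull direction blends in the actor's right vector scaled by left/right input, allowing sideways steering.
; UnGrab restores Walking and hides the cable; both events receive their movement component and cable as parameters.
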(event `Grab`
  (params (Movement :type "CharacterMovementComponent Object Reference") (Cable :type "CableComponent Object Reference") (Actor :type "Actor Object Reference") (GrabPoint :type "Vector Structure") (`Move Right/Left` :type "Float (double-precision)"))
  (`CharacterMovementComponent.SetMovementMode` Movement "MOVE_Flying" 0)
  (`SceneComponent.SetVisibility` Cable true false)
  (set `CableComponent.EndLocation` (`KismetMathLibrary.InverseTransformLocation` (`Actor.GetTransform` Actor) GrabPoint) Cable)
  (`CharacterMovementComponent.AddForce` Movement (* (`KismetMathLibrary.Normal` (+ (`KismetMathLibrary.GetDirectionUnitVector` (`Actor.K2_GetActorLocation` Actor) GrabPoint) (* (* (`Actor.GetActorRightVector` Actor) `Move Right/Left`) 0.7))) 10000000.0)))

(event `UnGrab`
  (params (Movement :type "CharacterMovementComponent Object Reference") (Cable :type "SceneComponent Object Reference"))
  (`CharacterMovementComponent.SetMovementMode` Movement "MOVE_Walking" 0)
  (`SceneComponent.SetVisibility` Cable false false))
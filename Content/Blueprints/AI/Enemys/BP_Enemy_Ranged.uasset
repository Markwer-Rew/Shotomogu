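; Ranged enemy that attacks the player by spawning a bullet actor.
; BeginPlay caches the player character as the target.
; Attack plays a punch montage and immediately spawns BP_TestBullet at the arrow component, passing it the player and an infinite damage-over-time gameplay effect class.
; Montage completion or interruption signals attack end, and GetIdealRage supplies fixed long-range attack and defend radii.
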(event `/Game/Blueprints/AI/BPI_EnemyAI.Attack`
  (`|PlayMontage` (`self.Mesh`) "/Game/Anims/MM_Punch.MM_Punch"
    (:`then`
      (`|SpawnActorFromClass` "/Game/Blueprints/BP_TestBullet.BP_TestBullet_C" (`SceneComponent.K2_GetComponentToWorld` (`self.Arrow1`)) "Undefined" "MultiplyWithRoot" null (`self.As BP Player Base`) "/Game/Blueprints/Effects/GE_DamageOverTime_Infinite.GE_DamageOverTime_Infinite_C" (struct) -15.0 null))
    (:`OnCompleted`
      (`self.OnAttackEnd` :!label _label))
    (:`OnInterrupted`
      (goto _label))))

(event `self.ReceiveBeginPlay`
  (bind _asbp_player_base (cast `/Game/Blueprints/Characters/BP_Player_Base` (`GameplayStatics.GetPlayerCharacter` 0)))
  (set `self.As BP Player Base` _asbp_player_base))

(fn `GetIdealRage`
  (returns (AttackRadius :type "Float (double-precision)") (DefendRadius :type "Float (double-precision)"))
  (return 1000.0 900.0))

(fn `UserConstructionScript`
  (`parent.UserConstructionScript`))
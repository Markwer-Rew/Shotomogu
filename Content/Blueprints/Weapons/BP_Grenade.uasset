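; BP_Grenade is a timed grenade weapon actor that deals area damage through an expanding collision volume.
; After BeginPlay and a delay, the Explosion timeline scales DamageCollision toward a large size, lerping from its current scale each update, then destroys the actor.
; Any actor that begins overlapping DamageCollision, except SoftRef, receives flat damage, with no check that the explosion has started.
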(event `self.ReceiveBeginPlay`
  (bind _damagecollision (`self.DamageCollision`))
  (bind (_returnvalue_x _returnvalue_y _returnvalue_z) (`KismetMathLibrary.BreakVector` (`SceneComponent.K2_GetComponentScale` _damagecollision)))
  (`KismetSystemLibrary.Delay` (`self.Duration`))
  (bind (_direction _time) (`Timeline|Explosion` :!via `PlayFromStart`)
    (:`Update`
      (`SceneComponent.SetWorldScale3D` _damagecollision (`KismetMathLibrary.MakeVector` (`KismetMathLibrary.Lerp` _returnvalue_x 15.0 _time) (`KismetMathLibrary.Lerp` _returnvalue_y 15.0 _time) (`KismetMathLibrary.Lerp` _returnvalue_z 15.0 _time))))
    (:`Finished`
      (`self.K2_DestroyActor`))))

(event `self.DamageCollision.OnComponentBeginOverlap`
  (params (OverlappedComponent :type "PrimitiveComponent Object Reference") (OtherActor :type "Actor Object Reference") (OtherComp :type "PrimitiveComponent Object Reference") (OtherBodyIndex :type Integer) (bFromSweep :type Boolean) (SweepResult :type "HitResult Structure (by ref)"))
  (if (!= OtherActor (`self.SoftRef`))
    (`GameplayStatics.ApplyDamage` OtherActor 45.0 null null "/Script/Engine.DamageType")))

(fn `UserConstructionScript`)
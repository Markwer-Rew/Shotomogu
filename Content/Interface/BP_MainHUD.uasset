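; BP_MainHUD is the game's main HUD Blueprint, which sets up the death screen and escape menu widgets.
; On BeginPlay it creates WBP_Dead and WBP_EscMenu, stores references to both, adds them to the viewport and leaves them hidden.
; Creation of the main widget, WBP_MainWIdget, is present but disconnected, so it never runs.
; The file contains no logic to show either hidden widget.
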(event `self.ReceiveBeginPlay`
  (`|ExecutionSequence`
    (:`then_1`
      (bind _returnvalue (`|CreateWidget` "/Game/Interface/WBP_Dead.WBP_Dead_C"))
      (bind _output_get (set `self.WBP_Dead` _returnvalue))
      (`UserWidget.AddToViewport` _returnvalue 0)
      (`UserWidget.AddToViewport` _output_get 0)
      (`Widget.SetVisibility` _returnvalue "Hidden")
      (`Widget.SetVisibility` _output_get "Hidden"))
    (:`then_2`
      (bind _returnvalue_2 (`|CreateWidget` "/Game/Interface/WBP_EscMenu.WBP_EscMenu_C"))
      (bind _output_get_2 (set `self.EscMenu` _returnvalue_2))
      (`UserWidget.AddToViewport` _output_get_2 0)
      (`Widget.SetVisibility` _output_get_2 "Hidden"))))

(fn `UserConstructionScript`)